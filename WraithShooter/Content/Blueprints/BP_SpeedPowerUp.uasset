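; Speed power-up Blueprint that temporarily doubles the walk speed of the player who activates it.
; OnActivated stores that player and sets their CharacterMovementComponent MaxWalkSpeed to twice GetMaxSpeed.
; OnExpired, if the stored player is still valid, sets it to half the current GetMaxSpeed rather than restoring a saved original.
; Activation and expiry timing are triggered outside these graphs.
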(event `self.OnActivated`
  (params (ActiveFor :type "Actor Object Reference"))
  (bind _returnvalue (`self.GetComponentByClass` ActiveFor "/Script/Engine.CharacterMovementComponent"))
  (set `self.Activated for player` ActiveFor)
  (set `CharacterMovementComponent.MaxWalkSpeed` (* (`MovementComponent.GetMaxSpeed` _returnvalue) 2.0) _returnvalue))

(event `self.OnExpired`
  (bind _activated_for_player (`self.Activated for player`))
  (bind _returnvalue (`self.GetComponentByClass` _activated_for_player "/Script/Engine.CharacterMovementComponent"))
  (`/Engine/EditorBlueprintResources/StandardMacros.IsValid` _activated_for_player
    (:`Is Valid`
      (set `CharacterMovementComponent.MaxWalkSpeed` (/ (`MovementComponent.GetMaxSpeed` _returnvalue) 2.0) _returnvalue))))

(fn `UserConstructionScript`
  (`parent.UserConstructionScript`))