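; BP_RegenPowerup is a powerup that heals the player's ShooterCharacter when activated.
; OnActivated stores the activating player but heals player pawn 0, provided its health and HealAmount are positive.
; The clamp takes health plus HealAmount as its minimum, so the heal is applied once and can exceed MaxHealth.
; It then prints HealAmount as debug output.
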(event `self.OnActivated`
  (params (ActiveFor :type "Actor Object Reference"))
  (bind _healamount (`self.HealAmount`))
  (set `self.ActivatedForPlayer` ActiveFor)
  (bind _asshooter_character (cast `ShooterCharacter` (`GameplayStatics.GetPlayerPawn` 0)))
  (bind _returnvalue (`ShooterCharacter.GetHealth` _asshooter_character))
  (if (not (or (<= _returnvalue 0.0) (<= _healamount 0.0)))
    (set `ShooterCharacter.Health` (`KismetMathLibrary.FClamp` _returnvalue (+ _returnvalue _healamount) (`ShooterCharacter.MaxHealth` _asshooter_character)) _asshooter_character)
    (`KismetSystemLibrary.PrintString` (`KismetStringLibrary.Conv_DoubleToString` (`self.HealAmount`)))))

(fn `UserConstructionScript`
  (`parent.UserConstructionScript`))