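; BP_ShooterPlayerController is a player controller that handles the offensive ability menu and dismissal of the learned-skill popup.
; It creates the menu widget on BeginPlay; holding the input swaps out the Wraith HUD, plays intro animation and sound, and pauses the game.
; Releasing restores the HUD and game-only input, with an extra sound if a selection was made.
; ExitSkillAquire removes the learned-skill widget and unpauses, only while paused.
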(event `InputAction|ExitSkillAquire` :consume false :paused true
  (params (Key :type "Key Structure"))
  (bind _returnvalue (`GameplayStatics.GetPlayerController` 0))
  ;[1 1 1] Hide AcquiredSkillWBP
  (:`Pressed`
    (if (`GameplayStatics.IsGamePaused`)
      (`Widget.RemoveFromParent` (`self.WBPLearnedSkill`))
      (`GameplayStatics.SetGamePaused` false)
      (`WidgetBlueprintLibrary.SetInputMode_GameOnly` _returnvalue)
      (set `PlayerController.bShowMouseCursor` false _returnvalue))))

(event `self.ReceiveBeginPlay`
  ;[1 1 1] Offensive Ability Menu Reference
  (bind _returnvalue (`|CreateWidget` "/Game/UI/WBP_OffensiveAbilityMenu.WBP_OffensiveAbilityMenu_C"))
  (set `self.OffensiveAbilityMenu` _returnvalue))

(event `InputAction|OffensiveAbilityMenu` :paused true
  (params (Key :type "Key Structure"))
  (bind _offensiveabilitymenu (`self.OffensiveAbilityMenu`))
  ;[1 1 1] Show/Hide Offensive Ability Menu
  (:`Pressed`
    (bind _asbp_wraith_hud (cast `/Game/Blueprints/BP_WraithHUD` (`self.GetHUD`)))
    (bind _hud (`WraithShooterHUD.HUD` _asbp_wraith_hud))
    (`Widget.RemoveFromParent` _hud)
    (`UserWidget.AddToViewport` _offensiveabilitymenu 0)
    (`UserWidget.PlayAnimation` _offensiveabilitymenu (`/Game/UI/WBP_OffensiveAbilityMenu.AbilityMenuIntro` _offensiveabilitymenu) 0.0 1 "Forward" 1.0 false)
    (`GameplayStatics.PlaySound2D` (`self.SFXMenu`) 1.0 1.0 0.0 null null)
    (`GameplayStatics.SetGamePaused` true)
    (`WidgetBlueprintLibrary.SetInputMode_GameAndUIEx` (`GameplayStatics.GetPlayerController` 0) (`self.OffensiveAbilityMenu`)))
  (:`Released`
    (`UserWidget.AddToViewport` _hud 0)
    (`Widget.RemoveFromParent` _offensiveabilitymenu)
    (`GameplayStatics.PlaySound2D` (`self.SFXMenuOff`) 1.0 1.0 0.0 null null)
    (`GameplayStatics.SetGamePaused` false)
    (`WidgetBlueprintLibrary.SetInputMode_GameOnly` (`GameplayStatics.GetPlayerController` 0))
    (if (`/Game/UI/WBP_OffensiveAbilityMenu.bSelectionMade?` (`self.OffensiveAbilityMenu`))
      (`GameplayStatics.PlaySound2D` "/Engine/VREditor/Sounds/VR_close_Cue.VR_close_Cue" 1.0 1.0 0.0 null null))))

(fn `UserConstructionScript`)